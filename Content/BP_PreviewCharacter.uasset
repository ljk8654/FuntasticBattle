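; BP_PreviewCharacter is a character Blueprint that configures physical animation on its skeletal mesh.
; On BeginPlay it binds the PhysicalAnimation component to Mesh and applies orientation, position, velocity and force-limit settings from the BodyName bone downward.
; It then sets those same bodies to not simulate physics, so the physical animation drive has no simulated bodies to act on there.
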(event EventBeginPlay
  (Class|PhysicalAnimationComponent|SetSkeletalMeshComponent (Variables|Default|GetPhysicalAnimation) (Variables|Character|GetMesh))
  (Class|PhysicalAnimationComponent|ApplyPhysicalAnimationSettingsBelow (Variables|Default|GetPhysicalAnimation) (Variables|Default|GetBody%20Name) (Utilities|Struct|MakePhysicalAnimationData true 1e+03 1e+02 1e+03 1e+02 1e+02 1e+02) true)
  (Class|SkeletalMeshComponent|SetAllBodiesBelowSimulatePhysics (Variables|Character|GetMesh) (Variables|Default|GetBody%20Name) false true))

(event Collision|EventActorBeginOverlap
  (params (OtherActor :type Actor%20Object%20Reference))
  (|CallParentFunction OtherActor) ; This node is disabled and will not be called.\nDrag off pins to build functionality.
)

(event EventTick
  (params (DeltaSeconds :type Float%20%28single-precision%29))
  (|CallParentFunction DeltaSeconds) ; This node is disabled and will not be called.\nDrag off pins to build functionality.
)

(fn ConstructionScript
  (|CallParentFunction))